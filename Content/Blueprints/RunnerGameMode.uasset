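; Game mode for a runner game that creates the HUD, sets Game and UI input, and builds an initial track of floor tiles on BeginPlay.
; AddFloorTile spawns a random straight tile, or randomly substitutes a corner through AddFloorCorner once enough straights have accumulated, resetting the count.
; Each spawned BP_FloorTile's attach transform becomes the next spawn point, chaining the track end to end.
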(event EventBeginPlay
  (Input|SetInputModeGameandUI (Game|GetPlayerController 0) 0 "DoNotLock" true)
  (bind _returnvalue (UserInterface|CreateWidget "/Game/UMG/RunnerHUD.RunnerHUD_C"))
  (UserInterface|Viewport|AddtoViewport _returnvalue 0)
  (for _index (range 0 19)
    (CallFunction|AddFloorTile)))

(fn ConstructionScript)

(fn AddFloorTile
  (bind _floortiles (Variables|Default|GetFloorTiles))
  (if (> (Variables|Default|GetCurrentStraights) 7)
    (if (== (Math|Random|RandomIntegerinRange 0 2) 2)
      (CallFunction|AddFloorCorner)
      (Variables|Default|SetCurrentStraights 0)
      (else
        (bind _returnvalue (Game|SpawnActorfromClass (Utilities|Array|Get(acopy) _floortiles (Math|Random|RandomIntegerinRange 0 (Utilities|Array|LastIndex _floortiles))) (Variables|Default|GetNextSpawnPoint) "AlwaysSpawn" 0 0 :!label _label))
        (bind _asbp_floor_tile (Utilities|Casting|CastToBP_FloorTile _returnvalue))
        (bind _attachtransform (Default|GetAttachTransform _asbp_floor_tile))
        (Variables|Default|SetNextSpawnPoint _attachtransform)
        (Math|Integer|IncrementInt (Variables|Default|GetCurrentStraights))))
    (else
      (goto _label))))

(fn AddFloorCorner
  (bind _floorcorner (Variables|Default|GetFloorCorner))
  (bind _returnvalue (Game|SpawnActorfromClass (Utilities|Array|Get(acopy) _floorcorner (Math|Random|RandomIntegerinRange 0 (Utilities|Array|LastIndex _floorcorner))) (Variables|Default|GetNextSpawnPoint) "Undefined" 0 0))
  (bind _asbp_floor_tile (Utilities|Casting|CastToBP_FloorTile _returnvalue))
  (bind _attachtransform (Default|GetAttachTransform _asbp_floor_tile))
  (Variables|Default|SetNextSpawnPoint _attachtransform))