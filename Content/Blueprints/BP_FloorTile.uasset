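; BP_FloorTile is a floor segment for an endless runner that exposes an attach transform, likely for chaining tiles.
; When the runner overlaps EndTrigger, it asks RunnerGameMode to add a tile, then destroys itself after a short delay.
; The DeathZone kills the runner, as do wall hits whose normal aligns with the runner's forward vector.
; Construction gathers three spawn points and randomly adds up to two blocker child actors via GetRandomSpawnPoint.
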(event OnComponentBeginOverlap(EndTrigger)
  (params (OverlappedComponent :type Primitive%20Component%20Object%20Reference) (OtherActor :type Actor%20Object%20Reference) (OtherComp :type Primitive%20Component%20Object%20Reference) (OtherBodyIndex :type Integer) (bFromSweep :type Boolean) (SweepResult :type Hit%20Result%20Structure%20%28by%20ref%29))
  (Utilities|Casting|CastToRunnerCharacter OtherActor)
  (bind _asrunner_game_mode (Utilities|Casting|CastToRunnerGameMode (Game|GetGameMode)))
  (Default|AddFloorTile _asrunner_game_mode)
  (Utilities|FlowControl|Delay 2.0)
  (Actor|DestroyActor))

(event OnComponentHit(Wall2)
  (params (HitComponent :type Primitive%20Component%20Object%20Reference) (OtherActor :type Actor%20Object%20Reference) (OtherComp :type Primitive%20Component%20Object%20Reference) (NormalImpulse :type Vector :default "0, 0, 0") (Hit :type Hit%20Result%20Structure%20%28by%20ref%29))
  (bind _asrunner_character (Utilities|Casting|CastToRunnerCharacter OtherActor))
  (if (Math|Float|NearlyEqual(Float) (Math|Vector|DotProduct (.normal Hit) (Transformation|GetActorForwardVector _asrunner_character)) 1.0 0.01)
    (Default|Death _asrunner_character)))

(event OnComponentHit(Wall)
  (params (HitComponent :type Primitive%20Component%20Object%20Reference) (OtherActor :type Actor%20Object%20Reference) (OtherComp :type Primitive%20Component%20Object%20Reference) (NormalImpulse :type Vector :default "0, 0, 0") (Hit :type Hit%20Result%20Structure%20%28by%20ref%29))
  (bind _asrunner_character (Utilities|Casting|CastToRunnerCharacter OtherActor))
  (if (Math|Float|NearlyEqual(Float) (Math|Vector|DotProduct (.normal Hit) (Transformation|GetActorForwardVector _asrunner_character)) 1.0 0.5)
    (Default|Death _asrunner_character)))

(event OnComponentBeginOverlap(DeathZone)
  (params (OverlappedComponent :type Primitive%20Component%20Object%20Reference) (OtherActor :type Actor%20Object%20Reference) (OtherComp :type Primitive%20Component%20Object%20Reference) (OtherBodyIndex :type Integer) (bFromSweep :type Boolean) (SweepResult :type Hit%20Result%20Structure%20%28by%20ref%29))
  (bind _asrunner_character (Utilities|Casting|CastToRunnerCharacter OtherActor))
  (Default|Death _asrunner_character))

(fn ConstructionScript
  (CallFunction|SetSpawnPoints)
  (switch int (Math|Random|RandomIntegerinRange 0 1)
    (:Default
      _)
    (:0
      _)
    (:1
      _))
  (CallFunction|SpawnBlocker))

(fn GetAttachTransform
  (return (Transformation|GetWorldTransform (Variables|Default|GetAttachPoint))))

(fn SetSpawnPoints
  (Variables|Default|SetSpawnPoints (Utilities|Array|MakeArray (Transformation|GetRelativeTransform (Variables|Default|GetSpawnPointL)) (Transformation|GetRelativeTransform (Variables|Default|GetSpawnPoint)) (Transformation|GetRelativeTransform (Variables|Default|GetSpawnPointR)))))

(fn SpawnBlocker
  (if (< (Math|Random|RandomIntegerinRange 0 100) 70)
    (AddComponent|AddChildActorComponent false (Utilities|GetRandomSpawnPoint))
    (if (< (Math|Random|RandomIntegerinRange 0 100) 30)
      (AddComponent|AddChildActorComponent false (Utilities|GetRandomSpawnPoint)))))